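; BP_Worker is a selectable worker unit that moves to target locations and gathers from resources.
; Select and deselect events toggle a selection decal, hidden on BeginPlay.
; MoveToTarget picks a navigable location from the target and uses simple AI movement.
; StartWorking stores the resource and starts a looping timer calling Work, which collects its held resources and updates that resource's progress.
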(event EventBeginPlay
  (Rendering|SetVisibility (Variables|Default|GetSelectionDecal) false false))

(event EventSelectUnit
  (Rendering|SetVisibility (Variables|Default|GetSelectionDecal) true false))

(event EventDeselectUnit
  (Rendering|SetVisibility (Variables|Default|GetSelectionDecal) false false))

(fn ConstructionScript)

(fn MovetoTarget
  (params (TargetLocation :type Vector))
  (bind _randomlocation (Class|NavigationSystemV1|GetRandomLocationinNavigableRadius TargetLocation 0.0 0 0))
  (AI|Navigation|SimpleMovetoLocation (Pawn|GetController) _randomlocation))

(fn StartWorking
  (params (Resource :type Interactable%20Resource%20Object%20Reference))
  (Variables|Default|SetCurrentResource Resource)
  (bind _returnvalue (Utilities|Time|SetTimerbyFunctionName 0 "Work" (Variables|Default|GetWorkingLoopDuration) true))
  (Variables|Default|SetWorkingTimerHandle _returnvalue))

(fn Work
  (Class|Worker|CollectResource (Variables|/Script/RTSBuildingManager.InteractableResource|GetHeldResources (Variables|Default|GetCurrentResource)))
  (Class|InteractableResource|UpdateCurrentResourceProgress (Variables|Default|GetCurrentResource)))