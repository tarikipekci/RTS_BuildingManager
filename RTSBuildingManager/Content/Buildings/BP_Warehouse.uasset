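; Warehouse building that goes through timed construction and takes collected resources from workers who reach it.
; StartBuilding shows a progress bar widget and starts a looping timer that advances it by the required build duration, then pauses, hides the widget and marks it built.
; Workers entering the interaction collision hand over resources and stop working, tracked in an overlap list to avoid repeat handling, without checking whether construction is finished.
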(event OnComponentBeginOverlap(InteractCollision)
  (params (OverlappedComponent :type Primitive%20Component%20Object%20Reference) (OtherActor :type Actor%20Object%20Reference) (OtherComp :type Primitive%20Component%20Object%20Reference) (OtherBodyIndex :type Integer) (bFromSweep :type Boolean) (SweepResult :type Hit%20Result%20Structure%20%28by%20ref%29))
  (bind _asbp_worker (Utilities|Casting|CastToBP_Worker OtherActor))
  (if (not (Utilities|Array|ContainsItem (Variables|Default|GetOverlappedWorkers) _asbp_worker))
    (Utilities|Array|Add (Variables|Default|GetOverlappedWorkers) _asbp_worker)
    (Class|WarehouseBuilding|TakeCollectedResources (Variables|/Script/RTSBuildingManager.Worker|GetCollectedResources _asbp_worker))
    (Variables|/Script/RTSBuildingManager.Worker|SetIsWorking _asbp_worker false)))

(event OnComponentEndOverlap(InteractCollision)
  (params (OverlappedComponent :type Primitive%20Component%20Object%20Reference) (OtherActor :type Actor%20Object%20Reference) (OtherComp :type Primitive%20Component%20Object%20Reference) (OtherBodyIndex :type Integer))
  (bind _asbp_worker (Utilities|Casting|CastToBP_Worker OtherActor))
  (Utilities|Array|RemoveItem (Variables|Default|GetOverlappedWorkers) _asbp_worker))

(event EventBeginPlay
  (Rendering|SetVisibility (Variables|Default|GetWidgetComp) false false))

(event EventStartBuilding
  (Rendering|SetVisibility (Variables|Default|GetWidgetComp) true false)
  (Utilities|Casting|CastToWBP_BuildingDuration (UserInterface|GetWidget (Variables|Default|GetWidgetComp)))
  (bind _returnvalue (Utilities|Time|SetTimerbyFunctionName 0 "UpdateBuildingProgress" 0.1 true))
  (Variables|Default|SetTimerHandle _returnvalue))

(fn ConstructionScript)

(fn UpdateBuildingProgress
  (bind _aswbp_building_duration (Utilities|Casting|CastToWBP_BuildingDuration (UserInterface|GetWidget (Variables|Default|GetWidgetComp))))
  (Variables|Default|SetPB_BuildingDuration (Variables|/Game/UI/Widgets/WBP_BuildingDuration.WBP_BuildingDuration_C|GetPB_Duration _aswbp_building_duration))
  (Variables|/Script/UMG.ProgressBar|SetPercent (Variables|Default|GetPB_BuildingDuration) (+ (Variables|/Script/UMG.ProgressBar|GetPercent (Variables|Default|GetPB_BuildingDuration)) (/ 0.1 (Variables|/Script/RTSBuildingManager.BuildingRequirements|GetBuildDuration (Variables|Default|GetRequirements)))))
  (if (>= (Variables|/Script/UMG.ProgressBar|GetPercent (Variables|Default|GetPB_BuildingDuration)) 1.0)
    (Utilities|Time|PauseTimerbyHandle (Variables|Default|GetTimerHandle))
    (Rendering|SetVisibility (Variables|Default|GetWidgetComp) false false)
    (Variables|Default|SetbBuilt true)))