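; Building actor that produces workers, with a timed construction phase and a click-to-open worker menu.
; StartBuilding shows a progress widget and starts a looping timer that fills its bar according to the required build duration.
; When the bar is full, the timer pauses, the widget hides and the building is marked built.
; Clicking a built, player-owned producer shows the HUD worker menu and registers it as selected in the GameState.
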(event EventBeginPlay
  (Rendering|SetVisibility (Variables|Default|GetWidgetComp) false false))

(event MouseInput|EventActorOnClicked
  (params (ButtonPressed :type Key%20Structure :default "None"))
  (if (Variables|Default|GetIsOwnerPlayer)
    (if (Variables|Default|GetbBuilt)
      (bind _asbp_hud (Utilities|Casting|CastToBP_HUD (HUD|GetHUD (Game|GetPlayerController 0))))
      (Variables|/Script/UMG.Widget|SetVisibility (Variables|/Game/UI/Widgets/WBP_WorkerMenu.WBP_WorkerMenu_C|GetListBorder (Variables|/Game/BP_HUD.BP_HUD_C|GetWorkerMenuWidget _asbp_hud)) "Visible")
      (bind _asbp_game_state (Utilities|Casting|CastToBP_GameState (Game|GetGameState)))
      (Variables|/Script/RTSBuildingManager.BuildingGameState|SetSelectedWorkerProducer _asbp_game_state self))))

(event EventStartBuilding
  (Rendering|SetVisibility (Variables|Default|GetWidgetComp) true false)
  (Utilities|Casting|CastToWBP_BuildingDuration (UserInterface|GetWidget (Variables|Default|GetWidgetComp)))
  (bind _returnvalue (Utilities|Time|SetTimerbyFunctionName 0 "UpdateBuildingProgress" 0.1 true))
  (Variables|Default|SetTimerHandle _returnvalue))

(fn ConstructionScript)

(fn UpdateBuildingProgress
  (bind _aswbp_building_duration (Utilities|Casting|CastToWBP_BuildingDuration (UserInterface|GetWidget (Variables|Default|GetWidgetComp))))
  (Variables|Default|SetPB_BuildingDuration (Variables|/Game/UI/Widgets/WBP_BuildingDuration.WBP_BuildingDuration_C|GetPB_Duration _aswbp_building_duration))
  (Variables|/Script/UMG.ProgressBar|SetPercent (Variables|Default|GetPB_BuildingDuration) (+ (Variables|/Script/UMG.ProgressBar|GetPercent (Variables|Default|GetPB_BuildingDuration)) (/ 0.1 (Variables|/Script/RTSBuildingManager.BuildingRequirements|GetBuildDuration (Variables|Default|GetRequirements)))))
  (if (>= (Variables|/Script/UMG.ProgressBar|GetPercent (Variables|Default|GetPB_BuildingDuration)) 1.0)
    (Utilities|Time|PauseTimerbyHandle (Variables|Default|GetTimerHandle))
    (Rendering|SetVisibility (Variables|Default|GetWidgetComp) false false)
    (Class|WorkerProducerBuilding|SetIsBuilt true)))