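; Gold producer building that shows construction and work progress through a WBP_BuildingDuration progress bar on its widget component, hidden at BeginPlay.
; StartBuilding runs a looping timer that fills the bar over the required build duration, then pauses it, hides the widget and calls StartWork.
; StartWorking shows the bar recolored and runs a second timer that refills it every work cycle.
; No gold is awarded in this graph.
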(event EventBeginPlay
  (Rendering|SetVisibility (Variables|Default|GetWidgetComp) false false))

(event EventStartWorking
  (Rendering|SetVisibility (Variables|Default|GetWidgetComp) true false)
  (Utilities|Casting|CastToWBP_BuildingDuration (UserInterface|GetWidget (Variables|Default|GetWidgetComp)))
  (bind _aswbp_building_duration (Utilities|Casting|CastToWBP_BuildingDuration (UserInterface|GetWidget (Variables|Default|GetWidgetComp))))
  (Progress|SetPercent (Variables|/Game/UI/Widgets/WBP_BuildingDuration.WBP_BuildingDuration_C|GetPB_Duration _aswbp_building_duration) 0.0)
  (bind _returnvalue (Utilities|Time|SetTimerbyFunctionName 0 "UpdateWorkingProgress" 0.1 true))
  (Variables|Default|SetTimerHandle _returnvalue)
  (Class|ProgressBar|SetFillColorandOpacity (Variables|Default|GetPB_BuildingDuration) "(R=0.000000,G=0.748598,B=0.864583,A=1.000000)"))

(event EventStartBuilding
  (Rendering|SetVisibility (Variables|Default|GetWidgetComp) true false)
  (Utilities|Casting|CastToWBP_BuildingDuration (UserInterface|GetWidget (Variables|Default|GetWidgetComp)))
  (bind _returnvalue (Utilities|Time|SetTimerbyFunctionName 0 "UpdateBuildingProgress" 0.1 true))
  (Variables|Default|SetTimerHandle _returnvalue))

(fn ConstructionScript)

(fn UpdateBuildingProgress
  (bind _aswbp_building_duration (Utilities|Casting|CastToWBP_BuildingDuration (UserInterface|GetWidget (Variables|Default|GetWidgetComp))))
  (Variables|Default|SetPB_BuildingDuration (Variables|/Game/UI/Widgets/WBP_BuildingDuration.WBP_BuildingDuration_C|GetPB_Duration _aswbp_building_duration))
  (Variables|/Script/UMG.ProgressBar|SetPercent (Variables|Default|GetPB_BuildingDuration) (+ (Variables|/Script/UMG.ProgressBar|GetPercent (Variables|Default|GetPB_BuildingDuration)) (/ 0.1 (Variables|/Script/RTSBuildingManager.BuildingRequirements|GetBuildDuration (Variables|Default|GetRequirements)))))
  (if (>= (Variables|/Script/UMG.ProgressBar|GetPercent (Variables|Default|GetPB_BuildingDuration)) 1.0)
    (Utilities|Time|PauseTimerbyHandle (Variables|Default|GetTimerHandle))
    (Rendering|SetVisibility (Variables|Default|GetWidgetComp) false false)
    (Class|GoldProducerBuilding|StartWork (Variables|/Script/RTSBuildingManager.BuildingRequirements|GetWorkDuration (Variables|Default|GetRequirements)))))

(fn UpdateWorkingProgress
  (bind _aswbp_building_duration (Utilities|Casting|CastToWBP_BuildingDuration (UserInterface|GetWidget (Variables|Default|GetWidgetComp))))
  (Variables|Default|SetPB_BuildingDuration (Variables|/Game/UI/Widgets/WBP_BuildingDuration.WBP_BuildingDuration_C|GetPB_Duration _aswbp_building_duration))
  (Variables|/Script/UMG.ProgressBar|SetPercent (Variables|Default|GetPB_BuildingDuration) (+ (Variables|/Script/UMG.ProgressBar|GetPercent (Variables|Default|GetPB_BuildingDuration)) (/ 0.1 (Variables|/Script/RTSBuildingManager.BuildingRequirements|GetWorkDuration (Variables|Default|GetRequirements)))))
  (if (>= (Variables|/Script/UMG.ProgressBar|GetPercent (Variables|Default|GetPB_BuildingDuration)) 1.0)
    (Variables|/Script/UMG.ProgressBar|SetPercent (Variables|Default|GetPB_BuildingDuration) 0.0)))