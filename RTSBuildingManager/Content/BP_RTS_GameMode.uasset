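; RTS game mode that sets up the building manager when play begins.
; BeginPlay spawns the BuildingManager class at the world origin, then casts the game state to BP_GameState and stores the manager in BuildingManagerRef if the cast succeeds.
; The same success path re-assigns the game state's CurrentBalance and the Buildables and Workers variables from identically named values.
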(event EventBeginPlay
  (bind _returnvalue (Game|SpawnActorfromClass "/Script/RTSBuildingManager.BuildingManager" (Math|Transform|MakeTransform "0, 0, 0") "Undefined" "MultiplyWithRoot" 0 0))
  (bind _asbp_game_state (Utilities|Casting|CastToBP_GameState (Game|GetGameState)))
  (Variables|/Script/RTSBuildingManager.BuildingGameState|SetCurrentBalance _asbp_game_state (Variables|/Script/RTSBuildingManager.BuildingGameState|GetCurrentBalance _asbp_game_state))
  (Variables|Default|SetBuildingManagerRef _returnvalue)
  (Variables|Default|SetBuildables (Variables|Default|GetBuildables))
  (Variables|Default|SetWorkers (Variables|Default|GetWorkers)))

(fn ConstructionScript)