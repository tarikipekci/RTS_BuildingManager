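; Behavior tree task that picks which building class the enemy AI should target next and writes it to the blackboard.
; It prioritizes a missing warehouse, then a missing worker producer, checking the enemy references on BP_GameState.
; With both present, it maps the blackboard resource type to the gold, wood or stone producer class.
; A resource type of None finishes successfully and leaves the building type unchanged.
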(event EventReceiveExecute
  (params (OwnerActor :type Actor%20Object%20Reference))
  (bind _bbkey_buildingtype (Variables|Default|GetBBKey_BuildingType))
  (bind _asbp_game_state (Utilities|Casting|CastToBP_GameState (Game|GetGameState)))
  (Utilities|IsValid (Variables|/Script/RTSBuildingManager.BuildingGameState|GetEnemyWarehouse _asbp_game_state)
    (:Is%20Valid
      (Utilities|IsValid (Variables|/Script/RTSBuildingManager.BuildingGameState|GetEnemyWorkerProducer _asbp_game_state)
        (:Is%20Valid
          (switch Utilities|FlowControl|Switch|SwitchonEResourceType (Utilities|Enum|ByteToEnumEResourceType (Class|BTFunctionLibrary|GetBlackboardValueasEnum (Variables|Default|GetBBKey_ResourceType)))
            (:None
              (AI|BehaviorTree|FinishExecute true))
            (:Gold
              (Class|BTFunctionLibrary|SetBlackboardValueasClass _bbkey_buildingtype "/Game/Buildings/BP_GoldProducer.BP_GoldProducer_C")
              (AI|BehaviorTree|FinishExecute true :!label _label))
            (:Log
              (Class|BTFunctionLibrary|SetBlackboardValueasClass _bbkey_buildingtype "/Game/Buildings/BP_WoodProducer.BP_WoodProducer_C")
              (goto _label))
            (:Stone
              (Class|BTFunctionLibrary|SetBlackboardValueasClass _bbkey_buildingtype "/Game/Buildings/BP_StoneProducer.BP_StoneProducer_C")
              (goto _label))))
        (:Is%20Not%20Valid
          (Class|BTFunctionLibrary|SetBlackboardValueasClass _bbkey_buildingtype "/Game/Buildings/BP_WorkerProducer.BP_WorkerProducer_C")
          (goto _label))))
    (:Is%20Not%20Valid
      (Class|BTFunctionLibrary|SetBlackboardValueasClass (Variables|Default|GetBBKey_BuildingType) "/Game/Buildings/BP_Warehouse.BP_Warehouse_C")
      (AI|BehaviorTree|FinishExecute true))))