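; Behavior tree task that spawns an enemy worker for the AI side while its worker count leads the ally count by less than two.
; It requires a valid enemy worker producer and consumes the AI resource cost from the worker class defaults.
; The worker spawns at a random navigable point near the producer, is possessed by a new AllyWorkerController, flagged non-ally and counted in the GameState.
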(event EventReceiveExecute
  (params (OwnerActor :type Actor%20Object%20Reference))
  (Variables|Default|SetWorkerClass "/Game/Workers/BP_Worker.BP_Worker_C")
  (bind _asbp_game_state (Utilities|Casting|CastToBP_GameState (Game|GetGameState)))
  (if (< (- (Variables|/Script/RTSBuildingManager.BuildingGameState|GetEnemyWorkerCount _asbp_game_state) (Variables|/Script/RTSBuildingManager.BuildingGameState|GetAllyWorkerCount _asbp_game_state)) 2)
    (bind _asbp_game_state_2 (Utilities|Casting|CastToBP_GameState (Game|GetGameState)))
    (bind _output_get (Variables|Default|SetGS _asbp_game_state_2))
    (Utilities|IsValid (Variables|/Script/RTSBuildingManager.BuildingGameState|GetEnemyWorkerProducer _output_get)
      (:Is%20Valid
        (bind _isthere (CallFunction|IsThereEnoughResources))
        (if _isthere
          (bind _returnvalue (Game|SpawnActorfromClass "/Script/RTSBuildingManager.AllyWorkerController" (Variables|Default|GetZeroLocation) "Undefined" "MultiplyWithRoot" 0 0))
          (Variables|Default|SetAIController _returnvalue)
          (bind _randomlocation (Class|NavigationSystemV1|GetRandomLocationinNavigableRadius (Transformation|GetActorLocation (Variables|/Script/RTSBuildingManager.BuildingGameState|GetEnemyWorkerProducer (Variables|Default|GetGS))) 2.5e+02 0 0))
          (bind _returnvalue_2 (Game|SpawnActorfromClass "/Game/Workers/BP_Worker.BP_Worker_C" (Math|Transform|MakeTransform _randomlocation) "Undefined" "MultiplyWithRoot" 0 0))
          (bind _output_get_2 (Variables|Default|SetSpawnedWorker _returnvalue_2))
          (Pawn|Possess (Variables|Default|GetAIController) _output_get_2)
          (Class|Worker|SetIsAlly (Variables|Default|GetSpawnedWorker) false)
          (Math|Integer|IncrementInt (Variables|/Script/RTSBuildingManager.BuildingGameState|GetEnemyWorkerCount (Variables|Default|GetGS))
            (:%20%20
              (AI|BehaviorTree|FinishExecute true)))
          (else
            (AI|BehaviorTree|FinishExecute true))))
      (:Is%20Not%20Valid
        (AI|BehaviorTree|FinishExecute true)))
    (else
      (AI|BehaviorTree|FinishExecute true))))

(fn IsThereEnoughResources
  (bind _returnvalue (Class|BuildingGameState|ConsumeAIResource (Variables|Default|GetGS) (Variables|/Script/RTSBuildingManager.WorkerRequirements|GetRequiredResource (.WorkerRequirements (Utilities|GetClassDefaults (Variables|Default|GetWorkerClass))))))
  (return _returnvalue))