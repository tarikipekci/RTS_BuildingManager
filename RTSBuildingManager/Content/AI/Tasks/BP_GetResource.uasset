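; Behavior tree task that sends idle non-ally workers to gather the least-stocked resource type, as named by a blackboard key.
; It loops over every BP_Worker, skips allies and busy ones, and picks a gold, log or stone actor via GetActorOfClass, not by proximity.
; PerformTask moves the worker to a random navigable point near that resource and flags it working.
; Every branch finishes with success, including inside the loop.
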(event EventReceiveExecute
  (params (OwnerActor :type Actor%20Object%20Reference))
  (bind _outactors (Actor|GetAllActorsOfClass "/Game/Workers/BP_Worker.BP_Worker_C"))
  (for _array_element _outactors
    (bind _output_get (Variables|Default|SetCurrentWorker _array_element))
    (if (Variables|/Script/RTSBuildingManager.Worker|GetIsAlly _array_element)
      (AI|BehaviorTree|FinishExecute true)
      (elif (Variables|/Script/RTSBuildingManager.Worker|GetIsWorking _output_get)
        (AI|BehaviorTree|FinishExecute true)
        (else
          (switch Utilities|FlowControl|Switch|SwitchonEResourceType (Utilities|Enum|ByteToEnumEResourceType (Class|BlackboardComponent|GetValueasEnum (AI|GetBlackboard OwnerActor) (Variables|Default|GetLeastResourceKey)))
            (:None
              (AI|BehaviorTree|FinishExecute true))
            (:Gold
              (bind _returnvalue (Actor|GetActorOfClass "/Game/Resources/BP_GoldResource.BP_GoldResource_C"))
              (CallFunction|PerformTask (Transformation|GetActorLocation _returnvalue))
              (AI|BehaviorTree|FinishExecute true :!label _label))
            (:Log
              (bind _returnvalue_2 (Actor|GetActorOfClass "/Game/Resources/BP_LogResorce.BP_LogResorce_C"))
              (CallFunction|PerformTask (Transformation|GetActorLocation _returnvalue_2))
              (goto _label))
            (:Stone
              (bind _returnvalue_3 (Actor|GetActorOfClass "/Game/Resources/BP_StoneResource.BP_StoneResource_C"))
              (CallFunction|PerformTask (Transformation|GetActorLocation _returnvalue_3))
              (goto _label)))))))
  (AI|BehaviorTree|FinishExecute true))

(fn PerformTask
  (params (ResourceLocation :type Vector))
  (bind _randomlocation (Class|NavigationSystemV1|GetRandomLocationinNavigableRadius ResourceLocation 2.5e+02 0 0))
  (Default|MovetoTarget (Variables|Default|GetCurrentWorker) _randomlocation)
  (Variables|/Script/RTSBuildingManager.Worker|SetIsWorking (Variables|Default|GetCurrentWorker) true))