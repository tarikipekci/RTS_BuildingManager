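; Stone resource node that selected workers gather from, with a widget bar showing how much remains.
; Clicking it sends selected BP_Workers to random navigable points nearby.
; Overlap registers a worker and starts its work; leaving removes it and clears its work timer.
; Progress updates consume held resources, set the bar against the starting total using the last entry's pre-consumption count, and destroy the node when an entry is empty.
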(event OnComponentBeginOverlap(OverlapCollision)
  (params (OverlappedComponent :type Primitive%20Component%20Object%20Reference) (OtherActor :type Actor%20Object%20Reference) (OtherComp :type Primitive%20Component%20Object%20Reference) (OtherBodyIndex :type Integer) (bFromSweep :type Boolean) (SweepResult :type Hit%20Result%20Structure%20%28by%20ref%29))
  (bind _asbp_worker (Utilities|Casting|CastToBP_Worker OtherActor))
  (if (not (Utilities|Array|ContainsItem (Variables|Default|GetCurrentWorkers) _asbp_worker))
    (Utilities|Array|Add (Variables|Default|GetCurrentWorkers) _asbp_worker)
    (Default|StartWorking _asbp_worker self)))

(event OnComponentEndOverlap(OverlapCollision)
  (params (OverlappedComponent :type Primitive%20Component%20Object%20Reference) (OtherActor :type Actor%20Object%20Reference) (OtherComp :type Primitive%20Component%20Object%20Reference) (OtherBodyIndex :type Integer))
  (bind _asbp_worker (Utilities|Casting|CastToBP_Worker OtherActor))
  (Utilities|Array|RemoveIndex (Variables|Default|GetCurrentWorkers) (Utilities|Array|FindItem (Variables|Default|GetCurrentWorkers) _asbp_worker))
  (Utilities|Time|ClearandInvalidateTimerbyHandle (Variables|/Game/Workers/BP_Worker.BP_Worker_C|GetWorkingTimerHandle _asbp_worker)))

(event EventBeginPlay
  (bind _aswbp_building_duration (Utilities|Casting|CastToWBP_BuildingDuration (UserInterface|GetWidget (Variables|Default|GetWidgetComp))))
  (Variables|/Script/UMG.ProgressBar|SetPercent (Variables|/Game/UI/Widgets/WBP_BuildingDuration.WBP_BuildingDuration_C|GetPB_Duration _aswbp_building_duration) 1.0)
  (CallFunction|FindMaxResourceCount))

(event EventUpdateCurrentResourceProgress
  (CallFunction|UpdateResourceAmount))

(event MouseInput|EventActorOnClicked
  (params (ButtonPressed :type Key%20Structure :default "None"))
  (bind _asbp_hud (Utilities|Casting|CastToBP_HUD (HUD|GetHUD (Game|GetPlayerController 0))))
  (for _array_element (Variables|/Game/BP_HUD.BP_HUD_C|GetSelectedUnits _asbp_hud)
    (bind _asbp_worker (Utilities|Casting|CastToBP_Worker _array_element))
    (bind _randomlocation (Class|NavigationSystemV1|GetRandomLocationinNavigableRadius (Transformation|GetActorLocation) 2e+02 0 0))
    (Default|MovetoTarget _asbp_worker _randomlocation)))

(fn ConstructionScript)

(fn UpdateResourceAmount
  (bind _aswbp_building_duration (Utilities|Casting|CastToWBP_BuildingDuration (UserInterface|GetWidget (Variables|Default|GetWidgetComp))))
  (Variables|Default|SetPB_Duration (Variables|/Game/UI/Widgets/WBP_BuildingDuration.WBP_BuildingDuration_C|GetPB_Duration _aswbp_building_duration))
  (bind _keys (Utilities|Map|Keys (Variables|Default|GetHeldResources)))
  (for _array_element _keys
    (bind _output_get (Variables|Default|SetTotalResourceCount (Math|Conversions|ToFloat(Integer) (+ (.Value (Utilities|Map|Find (Variables|Default|GetHeldResources) _array_element)) 0))))
    (if (<= _output_get 0.0)
      (Actor|DestroyActor)
      (else
        (Class|InteractableResource|ConsumeResources))))
  (Progress|SetPercent (Variables|Default|GetPB_Duration) (/ (Variables|Default|GetTotalResourceCount) (Variables|Default|GetMaxResourceSize)))
  (Variables|Default|SetTotalResourceCount 0.0))

(fn FindMaxResourceCount
  (bind _aswbp_building_duration (Utilities|Casting|CastToWBP_BuildingDuration (UserInterface|GetWidget (Variables|Default|GetWidgetComp))))
  (Variables|Default|SetPB_Duration (Variables|/Game/UI/Widgets/WBP_BuildingDuration.WBP_BuildingDuration_C|GetPB_Duration _aswbp_building_duration))
  (bind _keys (Utilities|Map|Keys (Variables|Default|GetHeldResources)))
  (for _array_element _keys
    (Variables|Default|SetMaxResourceSize (Math|Conversions|ToFloat(Integer) (+ (.Value (Utilities|Map|Find (Variables|Default|GetHeldResources) _array_element)) (Variables|Default|GetMaxResourceSize))))))