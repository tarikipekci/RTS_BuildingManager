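; BP_RTSController is the RTS player controller, showing the mouse cursor and handling unit orders.
; Holding R, despite the IsLeftMousePressed flag name, sends pressed, held and released messages to the HUD.
; Right-click projects the cursor onto the Z=0 plane, sends each selected BP_Worker to a random navigable point nearby and spawns one Niagara marker.
; Left-click hides the HUD's worker menu list unless a BP_WorkerProducer is under the cursor.
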(event EventBeginPlay
  (Variables|/Script/Engine.PlayerController|SetbShowMouseCursor (Game|GetPlayerController 0) true))

(event EventTick
  (params (DeltaSeconds :type Float%20%28single-precision%29))
  (if (Variables|Default|GetIsLeftMousePressed)
    (Class|RTSInterface|Held(Message) (HUD|GetHUD))))

(event Input|MouseEvents|RightMouseButton
  (params (Key :type Key%20Structure :default "None"))
  (bind (_worldlocation _worlddirection) (Game|Player|ConvertMouseLocationToWorldSpace))
  (bind _z (Math|Vector|BreakVector _worldlocation))
  (bind _z_2 (Math|Vector|BreakVector _worlddirection))
  (bind _returnvalue (/ _z _z_2))
  (bind _returnvalue_2 (* _worlddirection _returnvalue))
  (bind _returnvalue_3 (* _returnvalue_2 -1.0))
  (bind _returnvalue_4 (+ _worldlocation _returnvalue_3))
  (bind _returnvalue_5 (Math|Transform|MakeTransform _returnvalue_4))
  (bind _location (Math|Transform|BreakTransform _returnvalue_5))
  (:Pressed
    (Variables|Default|SetNiagaraSpawned false)
    (bind _asbp_hud (Utilities|Casting|CastToBP_HUD (HUD|GetHUD)))
    (for _array_element (Variables|/Game/BP_HUD.BP_HUD_C|GetSelectedUnits _asbp_hud)
      (bind _asbp_worker (Utilities|Casting|CastToBP_Worker _array_element))
      (bind _randomlocation (Class|NavigationSystemV1|GetRandomLocationinNavigableRadius _location 4e+02 0 0))
      (Default|MovetoTarget _asbp_worker _randomlocation)
      (if (not (Variables|Default|GetNiagaraSpawned))
        (Niagara|SpawnSystematLocation "/Game/Cursor/FX_Cursor.FX_Cursor" _location)
        (Variables|Default|SetNiagaraSpawned true)))))

(event Input|KeyboardEvents|R
  (params (Key :type Key%20Structure :default "None"))
  (bind _returnvalue (HUD|GetHUD))
  (:Pressed
    (Variables|Default|SetIsLeftMousePressed true)
    (Class|RTSInterface|Pressed(Message) _returnvalue))
  (:Released
    (Variables|Default|SetIsLeftMousePressed false)
    (Class|RTSInterface|Released(Message) _returnvalue)))

(event Input|MouseEvents|LeftMouseButton
  (params (Key :type Key%20Structure :default "None"))
  (:Pressed
    (bind _asbp_hud (Utilities|Casting|CastToBP_HUD (HUD|GetHUD)))
    (Utilities|Casting|CastToBP_WorkerProducer (.hitactor (.HitResult (Game|Player|GetHitResultUnderCursorbyChannel "TraceTypeQuery1" true)))
      (:CastFailed
        (Widget|SetVisibility (Variables|/Game/UI/Widgets/WBP_WorkerMenu.WBP_WorkerMenu_C|GetListBorder (Variables|/Game/BP_HUD.BP_HUD_C|GetWorkerMenuWidget _asbp_hud)) "Hidden")))))

(fn ConstructionScript)